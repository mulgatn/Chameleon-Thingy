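; Test Blueprint that detects the surface color under the player character and prints it on screen as debug text in that color.
; Each tick, a downward line trace finds the floor; landscape hits map the physical surface type to a color parameter of the landscape material.
; Other hits read the "Color" parameter from the material at the hit face.
; Both paths create dynamic material instances every tick to read these values.
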(event `self.ReceiveTick`
  (params (DeltaSeconds :type "Float (single-precision)"))
  (bind (_returnvalue_x _returnvalue_y _returnvalue_z) (`KismetMathLibrary.BreakVector` (`self.K2_GetActorLocation` (`GameplayStatics.GetPlayerCharacter` 0))))
  (bind _outhit (`KismetSystemLibrary.LineTraceSingle` :`Start` (`KismetMathLibrary.MakeVector` _returnvalue_x _returnvalue_y _returnvalue_z) :`End` (`KismetMathLibrary.MakeVector` _returnvalue_x _returnvalue_y (- _returnvalue_z 900.0)) :`TraceChannel` "TraceTypeQuery1" :`DrawDebugType` "ForDuration"))
  (`/Engine/EditorBlueprintResources/StandardMacros.IsValid` (`.HitActor` (`GameplayStatics.BreakHitResult` _outhit))
    (:`Is Valid`
      ;[0.9879 1 0.4779] Get color from landscape surfaces (could be optimized)
      (bind _aslandscape (cast `Landscape` (`.HitActor` (`GameplayStatics.BreakHitResult` _outhit)))
        (:`then`
          (bind _color (`self.Get Landscape Material Color` _aslandscape (`PhysicalMaterial.SurfaceType` (`.PhysMat` (`GameplayStatics.BreakHitResult` _outhit)))))
          ;[1 1 1] Debug
          (`KismetSystemLibrary.PrintString` (`KismetStringLibrary.Conv_ColorToString` _color) true true _color 0.0))
        (:`CastFailed`
          (bind (_sectionindex _returnvalue) (`PrimitiveComponent.GetMaterialFromCollisionFaceIndex` (`.HitComponent` (`GameplayStatics.BreakHitResult` _outhit)) (`.FaceIndex` (`GameplayStatics.BreakHitResult` _outhit))))
          ;[1 0.9577 0.4914] Get color from static mesh surfaces (could be optimized)
          (bind _returnvalue_2 (`PrimitiveComponent.CreateDynamicMaterialInstance` (`.HitComponent` (`GameplayStatics.BreakHitResult` _outhit)) _sectionindex _returnvalue "None"))
          (`/Engine/EditorBlueprintResources/StandardMacros.IsValid` _returnvalue_2
            (:`Is Valid`
              (bind _returnvalue_3 (`MaterialInstanceDynamic.K2_GetVectorParameterValue` _returnvalue_2 "Color"))
              ;[1 1 1] Debug
              (`KismetSystemLibrary.PrintString` (`KismetStringLibrary.Conv_ColorToString` _returnvalue_3) true true _returnvalue_3 0.0))))))))

(fn `Get Landscape Material Color`
  (params (Lanscape :type "Landscape Object Reference") (`Surface Type` :type "EPhysicalSurface Enum" :default "SurfaceType_Default"))
  (returns (Color :type "LinearColor Structure"))
  (bind _returnvalue (`KismetMaterialLibrary.CreateDynamicMaterialInstance` (`LandscapeProxy.LandscapeMaterial` Lanscape)))
  (bind _returnvalue_2 (`MaterialInstanceDynamic.K2_GetVectorParameterValue` _returnvalue "ColorSand"))
  (bind _returnvalue_3 (`MaterialInstanceDynamic.K2_GetVectorParameterValue` _returnvalue "ColorGrass"))
  (bind _returnvalue_4 (`MaterialInstanceDynamic.K2_GetVectorParameterValue` _returnvalue "ColorDarkGrass"))
  (bind _returnvalue_5 (`MaterialInstanceDynamic.K2_GetVectorParameterValue` _returnvalue "ColorRock"))
  (bind _returnvalue_6 (`MaterialInstanceDynamic.K2_GetVectorParameterValue` _returnvalue "ColorDarkSand"))
  (bind _returnvalue_7 (`MaterialInstanceDynamic.K2_GetVectorParameterValue` _returnvalue "ColorGround"))
  (return (select `EPhysicalSurface` `Surface Type` :`SurfaceType1` _returnvalue_2 :`SurfaceType2` _returnvalue_3 :`SurfaceType3` _returnvalue_4 :`SurfaceType4` _returnvalue_5 :`SurfaceType5` _returnvalue_7 :`SurfaceType6` _returnvalue_6)))

(fn `UserConstructionScript`)