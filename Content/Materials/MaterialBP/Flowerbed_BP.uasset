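; Flowerbed Blueprint that cycles its flower mesh through three colors over time.
; On BeginPlay it creates a dynamic instance of the windy masked flower material, applies it to the static mesh and starts a looping timer.
; Each timer tick plays a timeline that lerps the material's Color parameter from its current value to the next color.
; When the timeline finishes, the color index advances and wraps around.
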(event `self.ReceiveBeginPlay`
  (bind _returnvalue (`KismetMaterialLibrary.CreateDynamicMaterialInstance` "/Game/Materials/OBJECTS/FoliageMaterials/FlowerMaskedWindyBaseObject_MAT.FlowerMaskedWindyBaseObject_MAT"))
  (bind _output_get (set `self.materialReference` _returnvalue))
  (`PrimitiveComponent.SetMaterial` (`self.StaticMeshComponent`) 0 _output_get)
  (`KismetSystemLibrary.K2_SetTimerDelegate` (delegate `ChangeFlowerColor`) 8.0 true))

(event `ChangeFlowerColor`
  (bind _returnvalue (`MaterialInstanceDynamic.K2_GetVectorParameterValue` (`self.materialReference`) "Color"))
  (set `self.currentColor` _returnvalue)
  (set `self.newColor` (select `int` (`self.colorIndex`) :`0` (`self.Color1`) :`1` (`self.Color2`) :`2` (`self.Color3`)))
  (bind (_direction _alpha) (`Timeline|ColorChange` :!via `PlayFromStart`)
    (:`Update`
      (`MaterialInstanceDynamic.SetVectorParameterValue` (`self.materialReference`) "Color" (`KismetMathLibrary.LinearColorLerp` (`self.currentColor`) (`self.newColor`) _alpha)))
    (:`Finished`
      (bind _output_get (set `self.colorIndex` (+ (`self.colorIndex`) 1)))
      (if (> _output_get 2)
        (set `self.colorIndex` 0)))))

(fn `UserConstructionScript`)