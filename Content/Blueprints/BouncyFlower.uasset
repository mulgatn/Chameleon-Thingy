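; Bouncy flower prop that plays a close-then-reopen animation when the ThirdPersonCharacterCombined player overlaps its BouncyPart; no launch logic is in this graph.
; Two chained timelines drive three mesh morph targets, one inverted, with the closing timeline starting the opening one when it finishes.
; The construction script slightly randomizes mesh tilt and height and fully randomizes yaw, so placed copies vary.
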(event `self.BouncyPart.OnComponentBeginOverlap`
  (params (OverlappedComponent :type "PrimitiveComponent Object Reference") (OtherActor :type "Actor Object Reference") (OtherComp :type "PrimitiveComponent Object Reference") (OtherBodyIndex :type Integer) (bFromSweep :type Boolean) (SweepResult :type "HitResult Structure (by ref)"))
  (cast `/Game/GrapplingHook/ThirdPersonCharacterCombined` OtherActor)
  (`self.Close Flower`))

(event `Close Flower`
  (bind _bouncyflowermesh (`self.BouncyFlowerMesh`))
  (bind (_direction _alpha) (`Timeline|ClosingTime` :!via `PlayFromStart`)
    (:`Update`
      (`SkeletalMeshComponent.SetMorphTarget` _bouncyflowermesh "Lattice" _alpha true)
      (`SkeletalMeshComponent.SetMorphTarget` _bouncyflowermesh "SimpleDeform" _alpha true)
      (`SkeletalMeshComponent.SetMorphTarget` _bouncyflowermesh "Lattice_001" (* _alpha -1.0) true))
    (:`Finished`
      (`self.OpenFlower`))))

(event `OpenFlower`
  (bind _bouncyflowermesh (`self.BouncyFlowerMesh`))
  (bind (_direction _alpha) (`Timeline|OpeningTime` :!via `PlayFromStart`)
    (:`Update`
      (`SkeletalMeshComponent.SetMorphTarget` _bouncyflowermesh "Lattice" _alpha true)
      (`SkeletalMeshComponent.SetMorphTarget` _bouncyflowermesh "SimpleDeform" _alpha true)
      (`SkeletalMeshComponent.SetMorphTarget` _bouncyflowermesh "Lattice_001" (* _alpha -1.0) true))))

(fn `UserConstructionScript`
  (bind _bouncyflowermesh (`self.BouncyFlowerMesh`))
  (`SceneComponent.K2_SetRelativeRotation` _bouncyflowermesh (`KismetMathLibrary.MakeRotator` (`KismetMathLibrary.Conv_IntToDouble` (`KismetMathLibrary.RandomIntegerInRange` -5 5)) (`KismetMathLibrary.Conv_IntToDouble` (`KismetMathLibrary.RandomIntegerInRange` -5 5)) (`KismetMathLibrary.Conv_IntToDouble` (`KismetMathLibrary.RandomIntegerInRange` 0 360))) false false)
  (`SceneComponent.K2_SetRelativeLocation` _bouncyflowermesh (`KismetMathLibrary.MakeVector` 0.0 0.0 (`KismetMathLibrary.Conv_IntToDouble` (`KismetMathLibrary.RandomIntegerInRange` -6))) false false))