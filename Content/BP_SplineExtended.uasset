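; BP_SplineExtended is a construction-time spline mesh actor that lays a configurable static mesh along an editable spline.
; The construction script adds one SplineMeshComponent per segment, attached to the root and fitted to its two points' locations and tangents.
; It also carries each point's roll and Y/Z scale into the segment ends, so the mesh banks and tapers with the spline.
; Forward axis and collision type are variables; the event graph is empty.
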(fn `UserConstructionScript`
  (bind _spline (`self.Spline`))
  (for _index (range (+ (- (`SplineComponent.GetNumberOfSplinePoints` _spline) 2) 1))
    (bind _returnvalue (`AddComponent|NODE_AddSplineMeshComponent-0`))
    (`StaticMeshComponent.SetStaticMesh` _returnvalue (`self.Mesh`))
    (`SplineMeshComponent.SetForwardAxis` _returnvalue (`self.ForwardAxis`) true)
    (`SceneComponent.K2_AttachToComponent` _returnvalue (`self.DefaultSceneRoot`) "None" "KeepRelative" "KeepRelative" "KeepRelative" true)
    (bind (_location _tangent) (`SplineComponent.GetLocationAndTangentAtSplinePoint` _spline _index "Local"))
    (bind _returnvalue_2 (+ _index 1))
    (bind (_location_2 _tangent_2) (`SplineComponent.GetLocationAndTangentAtSplinePoint` _spline _returnvalue_2 "Local"))
    (`SplineMeshComponent.SetStartAndEnd` _returnvalue _location _tangent _location_2 _tangent_2 true)
    (bind _returnvalue_roll (`KismetMathLibrary.BreakRotator` (`SplineComponent.GetRotationAtSplinePoint` _spline _index "Local")))
    (`SplineMeshComponent.SetStartRoll` _returnvalue (`KismetMathLibrary.DegreesToRadians` _returnvalue_roll) false)
    (bind _returnvalue_roll_2 (`KismetMathLibrary.BreakRotator` (`SplineComponent.GetRotationAtSplinePoint` _spline _returnvalue_2 "Local")))
    (`SplineMeshComponent.SetEndRoll` _returnvalue (`KismetMathLibrary.DegreesToRadians` _returnvalue_roll_2) false)
    (bind (_returnvalue_x _returnvalue_y _returnvalue_z) (`KismetMathLibrary.BreakVector` (`SplineComponent.GetScaleAtSplinePoint` _spline _index)))
    (`SplineMeshComponent.SetStartScale` _returnvalue (`KismetMathLibrary.MakeVector2D` _returnvalue_y _returnvalue_z) false)
    (bind (_returnvalue_x_2 _returnvalue_y_2 _returnvalue_z_2) (`KismetMathLibrary.BreakVector` (`SplineComponent.GetScaleAtSplinePoint` _spline _returnvalue_2)))
    (`SplineMeshComponent.SetEndScale` _returnvalue (`KismetMathLibrary.MakeVector2D` _returnvalue_y_2 _returnvalue_z_2) true)
    (`PrimitiveComponent.SetCollisionEnabled` _returnvalue (`self.CollisionType`))))