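; Game mode Blueprint that respawns the player's ThirdPersonCharacterCombined after it is destroyed.
; BeginPlay and the Respawn event both bind OnDestroyed on the character of player index 0.
; On destruction, it waits briefly, spawns a new character at the stored SpawnTransform, possesses it with the player controller, then calls Respawn to rebind for the next death.
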(event `Respawn`
  (bind _asthird_person_character_combined (cast `/Game/GrapplingHook/ThirdPersonCharacterCombined` (`GameplayStatics.GetPlayerCharacter` 0) :!label _label))
  (add `Actor.OnDestroyed` _asthird_person_character_combined (delegate `OnDestroyed_`)))

(event `self.ReceiveBeginPlay`
  (goto _label))

(event `OnDestroyed_`
  (params (DestroyedActor :type "Actor Object Reference"))
  (`KismetSystemLibrary.Delay` 2.0)
  (bind _returnvalue (`|SpawnActorFromClass` "/Game/GrapplingHook/ThirdPersonCharacterCombined.ThirdPersonCharacterCombined_C" (`self.Spawn Transform`) "Undefined" "OverrideRootScale" null null))
  (`Controller.Possess` (`GameplayStatics.GetPlayerController` 0) _returnvalue)
  (`self.Respawn`))

(fn `UserConstructionScript`)