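; Respawn_BP is a checkpoint actor that sets the respawn position of the Cornelius character.
; Overlapping its Box stores Cornelius's current transform as RespawnPosition and flags the checkpoint as reached.
; Tick then shifts the PointLight toward blue with an HSV lerp and plays the checkpoint sound once.
; A Delay in Tick steps the lerp Alpha gradually, while the intensity and radius setters only reapply current values.
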(event `self.ReceiveTick`
  (params (DeltaSeconds :type "Float (single-precision)"))
  (bind _pointlight (`self.PointLight`))
  (bind _alpha (`self.Alpha`))
  (`|ExecutionSequence`
    (:`then_0`
      (if (`self.Checkpoint reached`)
        (`LightComponent.SetLightColor` _pointlight (`KismetMathLibrary.LinearColorLerpUsingHSV` (`LightComponentBase.GetLightColor` (`self.PointLight`)) (struct :`G` 0.554816 :`B` 0.973958 :`A` 1.0) (`self.Alpha`)) true)
        (`LightComponent.SetIntensity` _pointlight (`LightComponentBase.Intensity` _pointlight))
        (`LocalLightComponent.SetAttenuationRadius` _pointlight (`LocalLightComponent.AttenuationRadius` _pointlight))
        (`/Engine/EditorBlueprintResources/StandardMacros.DoOnce` false
          (:`Completed`
            (`GameplayStatics.PlaySoundAtLocation` "/Game/AI/NPC/NEW_SNAKE_AI/Checkpoint.Checkpoint" (`self.K2_GetActorLocation`) (struct) 1.0 1.0 0.0 null null null)))))
    (:`then_1`
      (if (`self.Checkpoint reached`)
        (`KismetSystemLibrary.Delay` 0.7)
        (if (<= _alpha 1.0)
          (set `self.Alpha` (+ _alpha 0.1)))))))

(event `self.Box.OnComponentBeginOverlap`
  (params (OverlappedComponent :type "PrimitiveComponent Object Reference") (OtherActor :type "Actor Object Reference") (OtherComp :type "PrimitiveComponent Object Reference") (OtherBodyIndex :type Integer) (bFromSweep :type Boolean) (SweepResult :type "HitResult Structure (by ref)"))
  (bind _ascornelius (cast `/Game/ThirdPersonCPP/Blueprints/Cornelius` OtherActor))
  (set `/Game/ThirdPersonCPP/Blueprints/Cornelius.Respawn Position` (`self.GetTransform` _ascornelius) _ascornelius)
  (set `self.Checkpoint reached` true))

(fn `UserConstructionScript`)